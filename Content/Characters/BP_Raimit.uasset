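; BP_Raimit is a character that turns to face the player and plays an attack animation when the player gets close.
; RangeSphere overlaps toggle TargetArea, which makes Tick yaw the mesh toward the player with a -90 degree offset.
; Entering AttaqueSphere sets AttaqueArea and plays the attack montage with a debug print, but applies no damage.
; A looping timer steadily drains CurrentHealth, with no death handling.
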(event OnComponentBeginOverlap(RangeSphere)
  (params (OverlappedComponent :type Primitive%20Component%20Object%20Reference) (OtherActor :type Actor%20Object%20Reference) (OtherComp :type Primitive%20Component%20Object%20Reference) (OtherBodyIndex :type Integer) (bFromSweep :type Boolean) (SweepResult :type Hit%20Result%20Structure%20%28by%20ref%29))
  (if (== OtherActor (Game|GetPlayerCharacter 0))
    (Variables|Default|SetTargetArea true)))

(event OnComponentEndOverlap(RangeSphere)
  (params (OverlappedComponent :type Primitive%20Component%20Object%20Reference) (OtherActor :type Actor%20Object%20Reference) (OtherComp :type Primitive%20Component%20Object%20Reference) (OtherBodyIndex :type Integer))
  (if (== OtherActor (Game|GetPlayerCharacter 0))
    (Variables|Default|SetTargetArea false)))

(event OnComponentBeginOverlap(AttaqueSphere)
  (params (OverlappedComponent :type Primitive%20Component%20Object%20Reference) (OtherActor :type Actor%20Object%20Reference) (OtherComp :type Primitive%20Component%20Object%20Reference) (OtherBodyIndex :type Integer) (bFromSweep :type Boolean) (SweepResult :type Hit%20Result%20Structure%20%28by%20ref%29))
  (if (== OtherActor (Game|GetPlayerCharacter 0))
    (Variables|Default|SetAttaqueArea true)
    (Animation|Montage|PlayMontage (Variables|Character|GetMesh) "/Game/Animations/AM_Attack_Montage.AM_Attack_Montage"
      (:then
        (Development|PrintString "Hello")))))

(event OnComponentEndOverlap(AttaqueSphere)
  (params (OverlappedComponent :type Primitive%20Component%20Object%20Reference) (OtherActor :type Actor%20Object%20Reference) (OtherComp :type Primitive%20Component%20Object%20Reference) (OtherBodyIndex :type Integer))
  (if (== OtherActor (Game|GetPlayerCharacter 0))
    (Variables|Default|SetAttaqueArea false)))

(event EventBeginPlay
  (Utilities|Time|SetTimerbyFunctionName 0 "LoseHealth" 0.5 true))

(event Collision|EventActorBeginOverlap
  (params (OtherActor :type Actor%20Object%20Reference)))

(event EventTick
  (params (DeltaSeconds :type Float%20%28single-precision%29))
  (if (Variables|Default|GetTargetArea)
    (Transformation|SetWorldRotation (Variables|Character|GetMesh) (Math|Rotator|MakeRotator 0.0 0.0 (- (.yaw (Math|Rotator|FindLookatRotation (Transformation|GetActorLocation) (Transformation|GetActorLocation (Game|GetPlayerCharacter 0)))) 9e+01)) false false)))

(fn ConstructionScript)

(fn LoseHealth
  (Variables|Default|SetCurrentHealth (- (Variables|Default|GetCurrentHealth) 1.0)))